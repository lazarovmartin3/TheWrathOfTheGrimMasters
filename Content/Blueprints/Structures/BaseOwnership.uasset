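; Capturable outpost that players and enemies take over by standing inside its Box trigger, with progress paused while both are present.
; Tick uses a one-second Delay to step a shared Timer, draining the opponent's ownership to neutral before filling toward the captor's own.
; Player overlap shows a BaseOwnershipHUD progress bar colored by owner.
; Player attacks on enemy-owned outposts alert the enemy through NotificationSystem using the outpost ID.
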(event `self.ReceiveBeginPlay`
  (bind _outactors (`GameplayStatics.GetAllActorsOfClass` "/Game/Level_BP/NotificationSystem.NotificationSystem_C"))
  (for _array_element _outactors
    (set `self.NotificationSm` _array_element)
    (set `self.timer` 0.5)))

(event `self.ReceiveTick`
  (params (DeltaSeconds :type "Float (single-precision)"))
  (bind _basehud (`self.BaseHUD`))
  (bind _timerimage (`/Game/HUD/BaseOwnershipHUD.TimerImage` _basehud))
  ;[1 1 1] Trigger
  (if (and (`self.PlayerIn`) (`self.EnemyIn`))
    _
    (elif (`self.PlayerIn`)
      ;[1 1 1] Player functions and updates
      (`KismetSystemLibrary.Delay` 1.0)
      (`self.PlayerTakingBase`)
      (if (`KismetSystemLibrary.IsValid` _basehud)
        (`ProgressBar.SetPercent` _timerimage (`self.timer`))
        (if (`self.EnemyOwn`)
          (`ProgressBar.SetFillColorAndOpacity` _timerimage (struct :`R` 0.697917 :`G` 0.014501 :`B` 0.021443 :`A` 1.0))
          (else
            (`ProgressBar.SetFillColorAndOpacity` _timerimage (struct :`G` 0.001323 :`B` 0.697917 :`A` 1.0))))
        (if (`self.PlayerOwn`)
          _))
      (elif (`self.EnemyIn`)
        (`KismetSystemLibrary.Delay` 1.0)
        (`self.EnemyTakingBase`)))))

(event `self.Box.OnComponentBeginOverlap`
  (params (OverlappedComponent :type "PrimitiveComponent Object Reference") (OtherActor :type "Actor Object Reference") (OtherComp :type "PrimitiveComponent Object Reference") (OtherBodyIndex :type Integer) (bFromSweep :type Boolean) (SweepResult :type "HitResult Structure (by ref)"))
  (bind _returnvalue (`self.ActorHasTag` OtherActor "Player"))
  (bind _returnvalue_2 (`self.ActorHasTag` OtherActor "Enemy"))
  ;[1 1 1] Both Are In
  (if (and _returnvalue _returnvalue_2)
    (set `self.PlayerIn` true)
    (set `self.EnemyIn` true)
    ;[1 1 1] Add The Proggress bar on the Screen
    (bind _returnvalue_3 (`|CreateWidget` "/Game/HUD/BaseOwnershipHUD.BaseOwnershipHUD_C" :!label _label))
    (bind _output_get (set `self.BaseHUD` _returnvalue_3))
    (`UserWidget.AddToViewport` _output_get 0)
    (bind _timerimage (`/Game/HUD/BaseOwnershipHUD.TimerImage` _output_get))
    (`ProgressBar.SetPercent` _timerimage (`self.timer`))
    (if (`self.EnemyOwn`)
      (`ProgressBar.SetFillColorAndOpacity` _timerimage (struct :`R` 0.697917 :`G` 0.014501 :`B` 0.021443 :`A` 1.0))
      (else
        (`ProgressBar.SetFillColorAndOpacity` _timerimage (struct :`G` 0.001323 :`B` 0.697917 :`A` 1.0))))
    (else
      ;[1 1 1] Only One is In
      (if _returnvalue
        (set `self.PlayerIn` true)
        (goto _label)
        (elif _returnvalue_2
          (set `self.EnemyIn` true))))))

(event `self.Box.OnComponentEndOverlap`
  (params (OverlappedComponent :type "PrimitiveComponent Object Reference") (OtherActor :type "Actor Object Reference") (OtherComp :type "PrimitiveComponent Object Reference") (OtherBodyIndex :type Integer))
  (if (`self.ActorHasTag` OtherActor "Player")
    (`Widget.RemoveFromParent` (`self.BaseHUD`))
    (set `self.PlayerIn` false))
  (if (`self.ActorHasTag` OtherActor "Enemy")
    (set `self.EnemyIn` false)))

(fn `EnemyTakingBase`
  (bind _timer (`self.timer`))
  (bind _timer_2 (`self.timer`))
  ;[1 1 1] Check if Enemy Own The Outpost
  (if (`self.PlayerOwn`)
    ;[1 1 1] Take From Player
    (if (> _timer 0.0)
      (set `self.timer` (- _timer 0.1))
      (if (<= _timer 0.05)
        (set `self.PlayerOwn` false)))
    (else
      ;[1 1 1] Player Own the Outpost
      (if (< _timer_2 1.0)
        (set `self.timer` (+ _timer_2 0.1))
        (if (>= _timer_2 0.98)
          (set `self.EnemyOwn` true))))))

(fn `PlayerTakingBase`
  (bind _timer (`self.timer`))
  (bind _timer_2 (`self.timer`))
  ;[1 1 1] Check if Enemy Own The Outpost
  (if (`self.EnemyOwn`)
    ;[1 1 1] Take From Enemy
    (`/Game/Level_BP/NotificationSystem.NotifyEnemy` (`self.NotificationSm`) (`self.ID`))
    (if (> _timer 0.0)
      (set `self.timer` (- _timer 0.1))
      (if (<= _timer 0.05)
        (set `self.EnemyOwn` false)))
    (else
      ;[1 1 1] Player Own the Outpost
      (if (< _timer_2 1.0)
        (set `self.timer` (+ _timer_2 0.1))
        (if (>= _timer_2 0.98)
          (set `self.PlayerOwn` true))))))

(fn `UserConstructionScript`)