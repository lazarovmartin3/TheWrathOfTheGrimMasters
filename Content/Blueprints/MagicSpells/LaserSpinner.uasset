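; LaserSpinner is a magic spell projectile actor that damages enemies it touches and destroys itself after a short delay.
; Each tick it moves the actor along EmptyMesh's forward vector by Speed and delta time, without sweep, taking rotation and scale from that mesh.
; Box overlaps apply fixed damage to actors tagged Enemy, and hits do not destroy the projectile.
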(event `self.ReceiveBeginPlay`
  (`KismetSystemLibrary.Delay` 3.0)
  (`self.K2_DestroyActor`))

(event `self.ReceiveTick`
  (params (DeltaSeconds :type "Float (single-precision)"))
  (`self.K2_SetActorTransform` (`KismetMathLibrary.MakeTransform` (+ (* (`SceneComponent.GetForwardVector` (`self.Empty_Mesh`)) (* (`GameplayStatics.GetWorldDeltaSeconds`) (`self.speed`))) (.location (`SceneComponent.K2_GetComponentToWorld` (`self.Empty_Mesh`)))) (.rotation (`SceneComponent.K2_GetComponentToWorld` (`self.Empty_Mesh`))) (.scale (`SceneComponent.K2_GetComponentToWorld` (`self.Empty_Mesh`))))))

(event `self.Box.OnComponentBeginOverlap`
  (params (OverlappedComponent :type "PrimitiveComponent Object Reference") (OtherActor :type "Actor Object Reference") (OtherComp :type "PrimitiveComponent Object Reference") (OtherBodyIndex :type Integer) (bFromSweep :type Boolean) (SweepResult :type "HitResult Structure (by ref)"))
  (if (`self.ActorHasTag` OtherActor "Enemy")
    (`GameplayStatics.ApplyDamage` OtherActor 20.0 null null "/Script/Engine.DamageType")))

(fn `UserConstructionScript`)