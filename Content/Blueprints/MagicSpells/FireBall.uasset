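; FireBall is a spell projectile actor that damages enemies on contact.
; On spawn it copies the player character's rotation, then each tick moves forward a fixed distance without sweeping, so its speed depends on frame rate.
; When its Collider overlaps an actor tagged Enemy, it applies the fireball damage read from the player character and destroys itself.
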(event `self.ReceiveBeginPlay`
  (`self.K2_SetActorRotation` (`self.K2_GetActorRotation` (`GameplayStatics.GetPlayerCharacter` 0))))

(event `self.ReceiveTick`
  (params (DeltaSeconds :type "Float (single-precision)"))
  (`self.K2_SetActorLocation` (+ (`self.K2_GetActorLocation`) (* (`KismetMathLibrary.GetForwardVector` (`self.K2_GetActorRotation`)) 20.0))))

(event `self.Collider.OnComponentBeginOverlap`
  (params (OverlappedComponent :type "PrimitiveComponent Object Reference") (OtherActor :type "Actor Object Reference") (OtherComp :type "PrimitiveComponent Object Reference") (OtherBodyIndex :type Integer) (bFromSweep :type Boolean) (SweepResult :type "HitResult Structure (by ref)"))
  (if (`self.ActorHasTag` OtherActor "Enemy")
    (`GameplayStatics.ApplyDamage` OtherActor (`Final_Year_ProjectCharacter.GetFireballDamage` (cast `Final_Year_ProjectCharacter` (`GameplayStatics.GetPlayerCharacter` 0) :!pure true)) null null "/Script/Engine.DamageType")
    (`self.K2_DestroyActor`)))

(fn `UserConstructionScript`)